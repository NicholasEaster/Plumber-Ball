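; Collectible coin for World 01 that spins and bobs until the player picks it up.
; Tick advances the yaw and adds an oscillating Z step to the location, reversing at set limits; both motions are per-frame, without delta time.
; When the player overlaps the Sphere, it increments CoinWorld01 in the GI_Persistance game instance and destroys itself.
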(event OnComponentBeginOverlap(Sphere)
  (params (OverlappedComponent :type Primitive%20Component%20Object%20Reference) (OtherActor :type Actor%20Object%20Reference) (OtherComp :type Primitive%20Component%20Object%20Reference) (OtherBodyIndex :type Integer) (bFromSweep :type Boolean) (SweepResult :type Hit%20Result%20Structure%20%28by%20ref%29))
  (Utilities|IsPlayer OtherActor
    (:IsPlayer
      ;[1 1 1] Add_Score_Value
      (bind _asgi_persistance (Utilities|Casting|CastToGI_Persistance (Game|GetGameInstance)))
      (Variables|/Game/Blueprint/GI_Persistance.GI_Persistance_C|SetCoin_World_01 _asgi_persistance (+ (Variables|/Game/Blueprint/GI_Persistance.GI_Persistance_C|GetCoin_World_01 _asgi_persistance) 1))
      (Actor|DestroyActor))))

(event EventTick
  (params (DeltaSeconds :type Float%20%28single-precision%29))
  (bind _returnvalue (Transformation|GetActorTransform))
  ;[1 1 1] Movement
  (bind _output_get (Variables|Default|SetCurrent_Rotation (+ (Variables|Default|GetCurrent_Rotation) 0.15)))
  (Transformation|SetActorRotation (Math|Rotator|MakeRotator 0.0 0.0 (Math|Float|%(Float) _output_get 3.6e+02)))
  (if (Variables|Default|Getup?)
    (if (>= (Variables|Default|GetCurrent_Transformation) 0.3)
      (Variables|Default|Setup? false)
      (else
        (bind _output_get_2 (Variables|Default|SetCurrent_Transformation (+ (Variables|Default|GetCurrent_Transformation) 0.0018)))))
    (Transformation|SetActorLocation (Math|Vector|MakeVector (.x (.location _returnvalue)) (.y (.location _returnvalue)) (+ (.z (.location _returnvalue)) _output_get_2)) false false)
    (else
      (if (<= (Variables|Default|GetCurrent_Transformation) -0.3)
        (Variables|Default|Setup? true)
        (else
          (bind _output_get_3 (Variables|Default|SetCurrent_Transformation (+ (Variables|Default|GetCurrent_Transformation) -0.0018)))))
      (Transformation|SetActorLocation (Math|Vector|MakeVector (.x (.location _returnvalue)) (.y (.location _returnvalue)) (+ _output_get_3 (.z (.location _returnvalue)))) false false))))

(fn ConstructionScript)