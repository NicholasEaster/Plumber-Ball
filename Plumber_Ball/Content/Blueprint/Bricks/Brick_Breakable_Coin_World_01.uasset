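; A breakable coin brick for World 01 that awards a coin when the player hits it.
; An overlap of its Box with BP_Player nudges the root component upward over a short MoveComponentTo.
; It then increments the CoinWorld01 count in the GI_Persistance game instance and destroys itself.
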(event OnComponentBeginOverlap(Box)
  (params (OverlappedComponent :type Primitive%20Component%20Object%20Reference) (OtherActor :type Actor%20Object%20Reference) (OtherComp :type Primitive%20Component%20Object%20Reference) (OtherBodyIndex :type Integer) (bFromSweep :type Boolean) (SweepResult :type Hit%20Result%20Structure%20%28by%20ref%29))
  (bind _defaultsceneroot (Variables|Default|GetDefaultSceneRoot))
  (bind _returnvalue (Transformation|GetRelativeTransform _defaultsceneroot))
  ;[1 1 1] Movement
  (Utilities|Casting|CastToBP_Player OtherActor)
  (Components|MoveComponentTo _defaultsceneroot (+ (.location _returnvalue) "0, 0,30.000000") (.rotation _returnvalue) false false 0.1 false)
  ;[1 1 1] Add_Score_Value
  (bind _asgi_persistance (Utilities|Casting|CastToGI_Persistance (Game|GetGameInstance)))
  (Variables|/Game/Blueprint/GI_Persistance.GI_Persistance_C|SetCoin_World_01 _asgi_persistance (+ (Variables|/Game/Blueprint/GI_Persistance.GI_Persistance_C|GetCoin_World_01 _asgi_persistance) 1))
  (Actor|DestroyActor))

(fn ConstructionScript)