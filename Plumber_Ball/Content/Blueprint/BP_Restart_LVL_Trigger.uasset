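; BP_Restart_LVL_Trigger is a fall-death trigger that restarts the current level when the player pawn overlaps it.
; On overlap it powers down BP_Player, shows the Fall_Death widget and fades the camera out.
; After the fade it adds the current game time to GI_Persistance's EnemyDeath and zeroes CoinWorld03, then reopens the level by name.
; BeginPlay fades the camera back in.
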(event OnComponentBeginOverlap(Trigger)
  (params (OverlappedComponent :type Primitive%20Component%20Object%20Reference) (OtherActor :type Actor%20Object%20Reference) (OtherComp :type Primitive%20Component%20Object%20Reference) (OtherBodyIndex :type Integer) (bFromSweep :type Boolean) (SweepResult :type Hit%20Result%20Structure%20%28by%20ref%29))
  ;[1 1 1] Check Overlap
  (if (== OtherActor (Game|Player|GetPlayerPawn 0))
    ;[1 1 1] Reset Size
    (bind _asbp_player (Utilities|Casting|CastToBP_Player OtherActor))
    (Default|PowerDown _asbp_player)
    ;[1 1 1] Death_Message
    (bind _returnvalue (UserInterface|CreateWidget "/Game/Text/Fall_Death.Fall_Death_C"))
    (UserInterface|Viewport|AddtoViewport _returnvalue 0)
    ;[1 1 1] Fade Out
    (CameraFades|StartCameraFade :self (Game|GetPlayerCameraManager 0) :ToAlpha 1.0 :Duration (Variables|Default|GetDuration) :bHoldWhenFinished true)
    (Utilities|FlowControl|Delay (Variables|Default|GetDuration))
    ;[1 1 1] Keep_Timing_And_Reset_Coins
    (bind _asgi_persistance (Utilities|Casting|CastToGI_Persistance (Game|GetGameInstance)))
    (Variables|/Game/Blueprint/GI_Persistance.GI_Persistance_C|SetEnemy%20Death _asgi_persistance (+ (Utilities|Time|GetGameTimeinSeconds) (Variables|/Game/Blueprint/GI_Persistance.GI_Persistance_C|GetEnemy%20Death _asgi_persistance)))
    (Variables|/Game/Blueprint/GI_Persistance.GI_Persistance_C|SetCoin_World_03 _asgi_persistance 0)
    ;[1 1 1] Restart Level
    (bind _returnvalue_2 (Game|GetCurrentLevelName true))
    (Game|OpenLevel(byName) (Utilities|String|StringToName _returnvalue_2))))

(event EventBeginPlay
  ;[1 1 1] Fade In
  (CameraFades|StartCameraFade :self (Game|GetPlayerCameraManager 0) :FromAlpha 1.0 :Duration (Variables|Default|GetDuration02)))

(fn ConstructionScript)