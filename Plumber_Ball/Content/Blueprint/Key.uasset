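; Collectible key that spins and bobs in place, then flies into the player when picked up.
; Tick applies fixed per-frame steps for yaw and a reversing vertical velocity, so idle motion depends on frame rate.
; A player overlap stores location, scale and light intensity, then the Collection timeline lerps toward the player while shrinking and dimming.
; A short delay on the timeline's Update destroys the actor; no inventory is updated here.
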(event OnComponentBeginOverlap(Sphere)
  (params (OverlappedComponent :type Primitive%20Component%20Object%20Reference) (OtherActor :type Actor%20Object%20Reference) (OtherComp :type Primitive%20Component%20Object%20Reference) (OtherBodyIndex :type Integer) (bFromSweep :type Boolean) (SweepResult :type Hit%20Result%20Structure%20%28by%20ref%29))
  (Utilities|IsPlayer OtherActor
    (:IsPlayer
      (CallFunction|StartingValues)
      ;[1 1 1] Animation
      (bind (_direction _collectionprogress _scaleprogress _lightintensity) (Timeline|Collection Play)
        (:Update
          (CallFunction|NewFunction0 _collectionprogress)
          (CallFunction|ScaletoPlayer _scaleprogress)
          (CallFunction|LightIntensityProgress _lightintensity)
          ;[1 1 1] Destroy_Key
          (Utilities|FlowControl|Delay 0.5)
          (Actor|DestroyActor))))))

(event EventTick
  (params (DeltaSeconds :type Float%20%28single-precision%29))
  (bind _returnvalue (Transformation|GetActorTransform))
  ;[1 1 1] Movement
  (bind _output_get (Variables|Default|SetCurrent%20Rotation (+ (Variables|Default|GetCurrent%20Rotation) 0.15)))
  (Transformation|SetActorRotation (Math|Rotator|MakeRotator 0.0 0.0 (Math|Float|%(Float) _output_get 3.6e+02)))
  (if (Variables|Default|Getup?)
    (if (>= (Variables|Default|GetCurrent%20Transformation) 0.3)
      (Variables|Default|Setup? false)
      (else
        (bind _output_get_2 (Variables|Default|SetCurrent%20Transformation (+ (Variables|Default|GetCurrent%20Transformation) 0.0018)))))
    (Transformation|SetActorLocation (Math|Vector|MakeVector (.x (.location _returnvalue)) (.y (.location _returnvalue)) (+ (.z (.location _returnvalue)) _output_get_2)) false false)
    (else
      (if (<= (Variables|Default|GetCurrent%20Transformation) -0.3)
        (Variables|Default|Setup? true)
        (else
          (bind _output_get_3 (Variables|Default|SetCurrent%20Transformation (+ (Variables|Default|GetCurrent%20Transformation) -0.0018)))))
      (Transformation|SetActorLocation (Math|Vector|MakeVector (.x (.location _returnvalue)) (.y (.location _returnvalue)) (+ _output_get_3 (.z (.location _returnvalue)))) false false))))

(fn ConstructionScript)

(fn NewFunction0
  (params (Alpha :type Float%20%28double-precision%29))
  (Transformation|SetActorLocation (Math|Vector|Lerp(Vector) (Variables|Default|GetCollectibleStartLocation) (Transformation|GetActorLocation (Game|Player|GetPlayerPawn 0)) Alpha) false false))

(fn StartingValues
  (Variables|Default|SetCollectibleStartLocation (Transformation|GetActorLocation))
  (Variables|Default|SetCollectibleStartScale (Transformation|GetActorScale3D))
  (Variables|Default|SetCollectibleStartIntensity (Variables|/Script/Engine.LightComponentBase|GetIntensity (Variables|Default|GetPointLight1))))

(fn ScaletoPlayer
  (params (Alpha :type Float%20%28double-precision%29))
  (Transformation|SetActorScale3D (Math|Vector|Lerp(Vector) (Variables|Default|GetCollectibleStartScale) "0, 0, 0" Alpha)))

(fn LightIntensityProgress
  (params (Alpha :type Float%20%28double-precision%29))
  (Rendering|Components|Light|SetIntensity (Variables|Default|GetPointLight1) (Math|Float|Lerp (Variables|Default|GetCollectibleStartIntensity) 0.0 Alpha)))