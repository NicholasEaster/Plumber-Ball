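; Player pawn for a rolling ball, driven by input-axis torque on the Sphere and an impulse jump rate-limited by the SpamRestriction macro.
; R toggles the view yaw by 180 degrees and inverts movement to match.
; PowerUp and PowerDown resize the ball, shift the camera height, record size in GI_Persistance, and toggle stronger torque and jump.
; BeginPlay fades in and adds Score and Time widgets outside the main menu.
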(event EventBeginPlay
  ;[1 1 1] Begin_Level
  (Pawn|Input|AddControllerYawInput 0.0)
  (Pawn|SetControlRotation (Game|GetPlayerController 0) (Math|Rotator|MakeRotator 0.0 -15.0 0.0))
  (CameraFades|StartCameraFade :self (Game|GetPlayerCameraManager 0) :FromAlpha 1.0 :Duration 2.0)
  (bind _asgi_persistance (Utilities|Casting|CastToGI_Persistance (Game|GetGameInstance)))
  (if (not (Variables|/Game/Blueprint/GI_Persistance.GI_Persistance_C|GetMain_Menu _asgi_persistance))
    (bind _returnvalue (UserInterface|CreateWidget "/Game/Text/Score.Score_C"))
    (UserInterface|Viewport|AddtoViewport _returnvalue 0)
    (bind _returnvalue_2 (UserInterface|CreateWidget "/Game/Text/Time.Time_C"))
    (UserInterface|Viewport|AddtoViewport _returnvalue_2 0)))

(event Input|ActionEvents|InputActionJump
  (params (Key :type Key%20Structure :default "None"))
  (bind _sphere (Variables|Default|GetSphere))
  ;[1 1 1] Movement
  (:Pressed
    (Utilities|SpamRestriction 1.5
      (:Spam%20Free
        (if (Variables|Default|GetPowered_Up)
          (Physics|AddImpulse _sphere (Math|Vector|MakeVector 0.0 0.0 (* 2.0 2.8e+05)) "None" false)
          (else
            (Physics|AddImpulse _sphere (Math|Vector|MakeVector 0.0 0.0 (* 1.0 2.8e+05)) "None" false)))))))

(event Input|AxisEvents|InputAxisMove_Forward/Backward
  (params (AxisValue :type Float%20%28single-precision%29))
  (bind _returnvalue (* -3.5e+07 AxisValue))
  (bind _returnvalue_2 (* AxisValue 3.5e+07))
  (bind _sphere (Variables|Default|GetSphere))
  (bind _sphere_2 (Variables|Default|GetSphere))
  ;[1 1 1] Movement
  (if (Variables|Default|GetInverted?)
    (if (Variables|Default|GetPowered_Up)
      (Class|PrimitiveComponent|AddTorqueinRadians _sphere (Math|Vector|MakeVector 0.0 (* _returnvalue 2.5) 0.0) "None" false)
      (else
        (Class|PrimitiveComponent|AddTorqueinRadians _sphere (Math|Vector|MakeVector 0.0 _returnvalue 0.0) "None" false)))
    (elif (Variables|Default|GetPowered_Up)
      (Class|PrimitiveComponent|AddTorqueinRadians _sphere_2 (Math|Vector|MakeVector 0.0 (* _returnvalue_2 2.5) 0.0) "None" false)
      (else
        (Class|PrimitiveComponent|AddTorqueinRadians _sphere_2 (Math|Vector|MakeVector 0.0 _returnvalue_2 0.0) "None" false)))))

(event Input|AxisEvents|InputAxisMove_Left/Right
  (params (AxisValue :type Float%20%28single-precision%29))
  (bind _returnvalue (* AxisValue -2e+07))
  (bind _returnvalue_2 (* AxisValue 2e+07))
  (bind _sphere (Variables|Default|GetSphere))
  ;[1 1 1] Movement
  (if (Variables|Default|GetInverted?)
    (if (Variables|Default|GetPowered_Up)
      (Class|PrimitiveComponent|AddTorqueinRadians _sphere (Math|Vector|MakeVector (* _returnvalue 2.5) 0.0 0.0) "None" false)
      (else
        (Class|PrimitiveComponent|AddTorqueinRadians _sphere (Math|Vector|MakeVector _returnvalue 0.0 0.0) "None" false)))
    (elif (Variables|Default|GetPowered_Up)
      (Class|PrimitiveComponent|AddTorqueinRadians _sphere (Math|Vector|MakeVector (* _returnvalue_2 2.5) 0.0 0.0) "None" false)
      (else
        (Class|PrimitiveComponent|AddTorqueinRadians _sphere (Math|Vector|MakeVector _returnvalue_2 0.0 0.0) "None" false)))))

(event Input|KeyboardEvents|R
  (params (Key :type Key%20Structure :default "None"))
  (:Pressed
    (if (Variables|Default|GetInverted?)
      (Pawn|Input|AddControllerYawInput 0.0)
      (Pawn|SetControlRotation (Game|GetPlayerController 0) (Math|Rotator|MakeRotator 0.0 -15.0 0.0))
      (Variables|Default|SetInverted? false)
      (else
        (Pawn|Input|AddControllerYawInput 0.0)
        (Pawn|SetControlRotation (Game|GetPlayerController 0) (Math|Rotator|MakeRotator 0.0 -15.0 1.8e+02))
        (Variables|Default|SetInverted? true)))))

(fn ConstructionScript)

(fn PowerUp
  (bind _camera (Variables|Default|GetCamera))
  (bind _returnvalue (Transformation|GetRelativeTransform _camera))
  (bind _asgi_persistance (Utilities|Casting|CastToGI_Persistance (Game|GetGameInstance)))
  (Variables|/Game/Blueprint/GI_Persistance.GI_Persistance_C|SetSize _asgi_persistance true)
  (Transformation|SetWorldScale3D (Variables|Default|GetSphere) "0.800000,0.800000,0.800000")
  (Variables|Default|SetCan%20Grow? true)
  (Variables|Default|SetPowered_Up true)
  (Transformation|SetRelativeTransform _camera (Math|Transform|MakeTransform (Math|Vector|MakeVector (.x (.location _returnvalue)) (.y (.location _returnvalue)) (+ (.z (.location _returnvalue)) 7e+01)) (.rotation _returnvalue) (.scale _returnvalue)) false false))

(fn PowerDown
  (bind _camera (Variables|Default|GetCamera))
  (bind _returnvalue (Transformation|GetRelativeTransform _camera))
  (bind _asgi_persistance (Utilities|Casting|CastToGI_Persistance (Game|GetGameInstance)))
  (Variables|/Game/Blueprint/GI_Persistance.GI_Persistance_C|SetSize _asgi_persistance false)
  (Transformation|SetWorldScale3D (Variables|Default|GetSphere) "0.600000,0.600000,0.600000")
  (Variables|Default|SetCan%20Grow? false)
  (Variables|Default|SetPowered_Up false)
  (Transformation|SetRelativeTransform _camera (Math|Transform|MakeTransform (Math|Vector|MakeVector (.x (.location _returnvalue)) (.y (.location _returnvalue)) (+ (.z (.location _returnvalue)) -7e+01)) (.rotation _returnvalue) (.scale _returnvalue)) false false))