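; Mushroom character that walks sideways as a Mario-style power-up for BP_Player.
; Tick feeds a WhereToGo direction into movement, which the Hit event flips along Y.
; Touching the player calls PowerUp and destroys the mushroom, unless CanGrow is true, which instead briefly switches capsule collision channel and physics.
; An Enemy Squish macro, unused in the event graph, halts movement, flattens the capsule and destroys the actor.
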(event OnComponentHit(CapsuleComponent)
  (params (HitComponent :type Primitive%20Component%20Object%20Reference) (OtherActor :type Actor%20Object%20Reference) (OtherComp :type Primitive%20Component%20Object%20Reference) (NormalImpulse :type Vector :default "0, 0, 0") (Hit :type Hit%20Result%20Structure%20%28by%20ref%29))
  (bind _capsulecomponent (Variables|Collision|GetCapsuleComponent))
  ;[1 1 1] Power_Up
  (bind _asbp_player (Utilities|Casting|CastToBP_Player OtherActor))
  (if (Variables|/Game/Blueprint/BP_Player.BP_Player_C|GetCan%20Grow? _asbp_player)
    ;[1 1 1] Stop Collisions
    (Collision|SetCollisionObjectType _capsulecomponent "ECC_GameTraceChannel1")
    (Physics|SetSimulatePhysics _capsulecomponent true)
    (Utilities|FlowControl|Delay 1.5)
    (Collision|SetCollisionObjectType _capsulecomponent "ECC_WorldDynamic")
    (Physics|SetSimulatePhysics _capsulecomponent false)
    ;[1 1 1] Set Rotation
    (Transformation|SetActorRotation (Math|Interpolation|RInterpTo (Transformation|GetActorRotation) "0, 0, 0" 1.0 1.0))
    (else
      (Default|PowerUp _asbp_player)
      (Actor|DestroyActor))))

(event EventTick
  (params (DeltaSeconds :type Float%20%28single-precision%29))
  ;[1 1 1] Movement
  (Pawn|Input|AddMovementInput (Variables|Default|GetWhere%20to%20go) 0.5 false))

(event Collision|EventHit
  (params (MyComp :type Primitive%20Component%20Object%20Reference) (Other :type Actor%20Object%20Reference) (OtherComp :type Primitive%20Component%20Object%20Reference) (bSelfMoved :type Boolean) (HitLocation :type Vector :default "0, 0, 0") (HitNormal :type Vector :default "0, 0, 0") (NormalImpulse :type Vector :default "0, 0, 0") (Hit :type Hit%20Result%20Structure%20%28by%20ref%29))
  ;[1 1 1] Movement
  (Utilities|FlowControl|FlipFlop
    (:A
      (Variables|Default|SetWhere%20to%20go "0,-1.000000, 0"))
    (:B
      (Variables|Default|SetWhere%20to%20go "0,1.000000, 0"))))

(fn ConstructionScript)