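; End-of-level trigger for Level 03 that opens the locked door when the player overlaps its capsule.
; HaveKey returns true while any Key actors remain in the level, in which case the overlap shows a Key widget instead.
; Otherwise, it destroys Locked_Door actors and its own StaticMesh3 once, then clears StopTime and saves game time as World03Time in GI_Persistance.
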(event OnComponentBeginOverlap(Capsule)
  (params (OverlappedComponent :type Primitive%20Component%20Object%20Reference) (OtherActor :type Actor%20Object%20Reference) (OtherComp :type Primitive%20Component%20Object%20Reference) (OtherBodyIndex :type Integer) (bFromSweep :type Boolean) (SweepResult :type Hit%20Result%20Structure%20%28by%20ref%29))
  ;[1 1 1] Open_Door
  (Utilities|IsPlayer OtherActor
    (:IsPlayer
      (if (CallFunction|HaveKey?)
        (bind _returnvalue (UserInterface|CreateWidget "/Game/Text/Key.Key_C"))
        (UserInterface|Viewport|AddtoViewport _returnvalue 0)
        (else
          (Utilities|FlowControl|DoOnce false
            (:Completed
              (bind _outactors (Actor|GetAllActorsOfClass "/Game/Blueprint/Locked_Door.Locked_Door_C"))
              (Actor|DestroyActor _outactors)
              ;[1 1 1] Get_Game_Time
              (Components|DestroyComponent (Variables|Default|GetStaticMesh3))
              (bind _asgi_persistance (Utilities|Casting|CastToGI_Persistance (Game|GetGameInstance)))
              (Variables|/Game/Blueprint/GI_Persistance.GI_Persistance_C|SetStop_Time _asgi_persistance false)
              (Variables|/Game/Blueprint/GI_Persistance.GI_Persistance_C|SetWorld_03Time _asgi_persistance (Utilities|Time|GetGameTimeinSeconds)))))))))

(fn ConstructionScript)

(fn HaveKey?
  (bind _outactors (Actor|GetAllActorsOfClass "/Game/Blueprint/Key.Key_C"))
  (return (> (Utilities|Array|Length _outactors) 0)))