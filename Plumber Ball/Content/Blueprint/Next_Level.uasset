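; Level-exit actor that advances the game to the next level when another actor overlaps it.
; CompleteLvl looks up the current level name in the LevelNames array and opens the following entry unless it is the last.
; The overlap then runs a DoOnce-guarded end sequence, adding win, coin, time, transition and score widgets to the viewport, spaced by delays.
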(event Collision|EventActorBeginOverlap
  (params (OtherActor :type Actor%20Object%20Reference))
  ;[1 1 1] Load_Next_Level
  (CallFunction|CompleteLvl)
  ;[1 1 1] Final_Score
  (Utilities|FlowControl|DoOnce false
    (:Completed
      (bind _returnvalue (UserInterface|CreateWidget "/Game/Text/You_WIn.You_WIn_C"))
      (UserInterface|Viewport|AddtoViewport _returnvalue 0)
      (Utilities|FlowControl|Delay 2.0)
      (bind _returnvalue_2 (UserInterface|CreateWidget "/Game/Text/Final_Coins.Final_Coins_C"))
      (UserInterface|Viewport|AddtoViewport _returnvalue_2 0)
      (Utilities|FlowControl|Delay 2.0)
      (bind _returnvalue_3 (UserInterface|CreateWidget "/Game/Text/Final_Time.Final_Time_C"))
      (UserInterface|Viewport|AddtoViewport _returnvalue_3 0)
      (Utilities|FlowControl|Delay 2.75)
      (bind _returnvalue_4 (UserInterface|CreateWidget "/Game/Text/Final_Transition.Final_Transition_C"))
      (UserInterface|Viewport|AddtoViewport _returnvalue_4 0)
      (Utilities|FlowControl|Delay 2.0)
      (bind _returnvalue_5 (UserInterface|CreateWidget "/Game/Text/Final_Score.Final_Score_C"))
      (UserInterface|Viewport|AddtoViewport _returnvalue_5 0))))

(fn ConstructionScript)

(fn CompleteLvl
  (if (CallFunction|IsFinalLevel?)
    (Utilities|FlowControl|DoOnce true)
    (else
      (Game|OpenLevel(byName) (Utilities|Array|Get(acopy) (Variables|Default|GetLevel%20Names) (+ (CallFunction|GetCurrentLevelIndex) 1))))))

(fn GetCurrentLevelIndex
  (bind _returnvalue (Game|GetCurrentLevelName true))
  (return (Utilities|Array|FindItem (Variables|Default|GetLevel%20Names) (Utilities|String|StringToName _returnvalue))))

(fn IsFinalLevel?
  (return (== (Utilities|Array|LastIndex (Variables|Default|GetLevel%20Names)) (CallFunction|GetCurrentLevelIndex))))