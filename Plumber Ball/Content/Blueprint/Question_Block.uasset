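; Question block actor that releases a mushroom when the player touches its trigger, like a Mario-style item block.
; A Box overlap by BP_Player nudges the root upward with a short MoveComponentTo.
; It then spawns a Mushroom with its default controller at the Arrow's transform.
; An Empty_Block spawns at the mesh's transform, and the question block destroys itself.
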(event OnComponentBeginOverlap(Box)
  (params (OverlappedComponent :type Primitive%20Component%20Object%20Reference) (OtherActor :type Actor%20Object%20Reference) (OtherComp :type Primitive%20Component%20Object%20Reference) (OtherBodyIndex :type Integer) (bFromSweep :type Boolean) (SweepResult :type Hit%20Result%20Structure%20%28by%20ref%29))
  (bind _defaultsceneroot (Variables|Default|GetDefaultSceneRoot))
  (bind _returnvalue (Transformation|GetRelativeTransform _defaultsceneroot))
  ;[1 1 1] Move_Up
  (Utilities|Casting|CastToBP_Player OtherActor)
  (Components|MoveComponentTo _defaultsceneroot (+ (.location _returnvalue) "0, 0,10.000000") (.rotation _returnvalue) false false 0.1 false)
  ;[1 1 1] Spawn_Actors
  (bind _returnvalue_2 (Game|SpawnActorfromClass "/Game/Blueprint/Mushroom.Mushroom_C" (Transformation|GetWorldTransform (Variables|Default|GetArrow)) "Undefined" 0 0))
  (Pawn|SpawnDefaultController _returnvalue_2)
  (Game|SpawnActorfromClass "/Game/Blueprint/Empty_Block.Empty_Block_C" (Transformation|GetWorldTransform (Variables|Default|GetStaticMesh)) "Undefined" 0 0)
  (Actor|DestroyActor))

(fn ConstructionScript)